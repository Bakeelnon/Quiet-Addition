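; Arena spawner Blueprint that continuously spawns red, blue, yellow and green enemies at random points.
; Tick drives a Sequence with a separate Delay per enemy type, so each type repeats on its own interval, with red the most frequent.
; Each spawn takes its location from GetRandomPoint and passes a matching color to the new enemy.
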(event EventTick
  (params (DeltaSeconds :type Float%20%28single-precision%29))
  (bind _returnvalue (Class|NavigationSystem|GetRandomPoint))
  (bind _returnvalue_2 (* _returnvalue "1.000000,1.000000,1.000000"))
  (bind _returnvalue_3 (Math|Transform|MakeTransform _returnvalue_2))
  (Utilities|FlowControl|Sequence
    (:then_0
      (Utilities|FlowControl|Delay 1.0)
      (Game|SpawnActorfromClass "/Game/Enemies/Blueprints/RedEnemy.RedEnemy_C" _returnvalue_3 false 0 "(R=1.000000,G=0.005134,B=0.000000,A=1.000000)" 0))
    (:then_1
      (Utilities|FlowControl|Delay 4.0)
      (Game|SpawnActorfromClass "/Game/Enemies/Blueprints/BlueEnemy.BlueEnemy_C" _returnvalue_3 false 0 "(R=0.000000,G=0.087874,B=1.000000,A=1.000000)" 0))
    (:then_2
      (Utilities|FlowControl|Delay 3.0)
      (Game|SpawnActorfromClass "/Game/Enemies/Blueprints/YellowEnemy.YellowEnemy_C" _returnvalue_3 false 0 "(R=1.000000,G=0.930940,B=0.000000,A=1.000000)" 0))
    (:then_3
      (Utilities|FlowControl|Delay 4.0)
      (Game|SpawnActorfromClass "/Game/Enemies/Blueprints/GreenEnemy.GreenEnemy_C" _returnvalue_3 false 0 "(R=0.178061,G=1.000000,B=0.000000,A=1.000000)" 0))))

(fn ConstructionScript)